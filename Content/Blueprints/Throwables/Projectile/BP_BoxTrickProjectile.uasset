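; Throwable trick-box projectile that drives its sprite, audio and lifetime from recharge, ready and activation events bound on BeginPlay.
; Recharge starts a looping timer that flip-flops between inactive and tick sprites to blink, and ready clears it, restoring the inactive sprite.
; Activation shows the active sprite, plays the spider-box (Caja_Araña) 2D audio event and destroys the actor after a short delay.
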(event Custom|TickLights
  (bind _returnvalue (Utilities|Time|SetTimerbyEvent (delegate Custom|TickTak) 0.25 true))
  (Variables|Default|SetTickImage _returnvalue))

(event Custom|TickTak
  (Utilities|FlowControl|FlipFlop
    (:A
      (Rendering|Components|Sprite|SetSprite (Variables|Default|GetPaperSprite) "/Game/Art/Throwables/BoxInactive_Sprite.BoxInactive_Sprite"))
    (:B
      (Rendering|Components|Sprite|SetSprite (Variables|Default|GetPaperSprite) "/Game/Art/Throwables/BoxInactiveTick_Sprite.BoxInactiveTick_Sprite"))))

(event Custom|CustomEvent
  (Utilities|Time|ClearandInvalidateTimerbyHandle (Variables|Default|GetTickImage))
  (Rendering|Components|Sprite|SetSprite (Variables|Default|GetPaperSprite) "/Game/Art/Throwables/BoxInactive_Sprite.BoxInactive_Sprite"))

(event Custom|OnActivated
  (Rendering|Components|Sprite|SetSprite (Variables|Default|GetPaperSprite) "/Game/Art/Throwables/BoxActive_Sprite.BoxActive_Sprite")
  (Class|FMODBlueprintStatics|PlayEvent2D "/Game/FMOD/Events/SFX/Caja_Araña.Caja_Araña")
  (Utilities|FlowControl|Delay 2.0)
  (Actor|DestroyActor))

(event EventBeginPlay
  (EventDispatchers|BindEventtoOnRechargeStarts (delegate Custom|TickLights))
  (EventDispatchers|BindEventtoOnReadyStarts (delegate Custom|CustomEvent))
  (EventDispatchers|BindEventtoOnBoxActivated (delegate Custom|OnActivated)))

(event Collision|EventActorBeginOverlap
  (params (OtherActor :type Actor%20Object%20Reference)))

(event EventTick
  (params (DeltaSeconds :type Float%20%28single-precision%29)))

(fn ConstructionScript)