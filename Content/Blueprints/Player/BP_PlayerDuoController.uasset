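; Player controller that runs two local players from a single controller, with both viewed through a shared camera.
; On BeginPlay it adds the game mapping context, spawns both player pawns and sets the view target to BP_InteligentCamera.
; Separate P1 and P2 input actions forward move, jump and interact to per-player functions defined outside this graph, with jump stop bound to Canceled.
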(event Input|EnhancedActionEvents|EnhancedInputActionI_InteractP1
  (params (ActionValue :type Boolean) (ElapsedSeconds :type Float%20%28double-precision%29) (TriggeredSeconds :type Float%20%28double-precision%29) (InputAction :type Input%20Action%20Object%20Reference :default "/Game/Blueprints/Player/Input/Player1/I_InteractP1.I_InteractP1"))
  (:Started
    (Class|PlayerDuoController|InteractP1)))

(event Input|EnhancedActionEvents|EnhancedInputActionI_InteractP2
  (params (ActionValue :type Boolean) (ElapsedSeconds :type Float%20%28double-precision%29) (TriggeredSeconds :type Float%20%28double-precision%29) (InputAction :type Input%20Action%20Object%20Reference :default "/Game/Blueprints/Player/Input/Player2/I_InteractP2.I_InteractP2"))
  (:Started
    (Class|PlayerDuoController|InteractP2)))

(event Input|EnhancedActionEvents|EnhancedInputActionI_MoveRightP1
  (params (ActionValue :type Float%20%28double-precision%29) (ElapsedSeconds :type Float%20%28double-precision%29) (TriggeredSeconds :type Float%20%28double-precision%29) (InputAction :type Input%20Action%20Object%20Reference :default "/Game/Blueprints/Player/Input/Player1/I_MoveRightP1.I_MoveRightP1"))
  (:Triggered
    (Class|PlayerDuoController|MoveRightP1 ActionValue)))

(event Input|EnhancedActionEvents|EnhancedInputActionI_MoveRightP2
  (params (ActionValue :type Float%20%28double-precision%29) (ElapsedSeconds :type Float%20%28double-precision%29) (TriggeredSeconds :type Float%20%28double-precision%29) (InputAction :type Input%20Action%20Object%20Reference :default "/Game/Blueprints/Player/Input/Player2/I_MoveRightP2.I_MoveRightP2"))
  (:Triggered
    (Class|PlayerDuoController|MoveRightP2 ActionValue)))

(event Input|EnhancedActionEvents|EnhancedInputActionI_JumpP1
  (params (ActionValue :type Boolean) (ElapsedSeconds :type Float%20%28double-precision%29) (TriggeredSeconds :type Float%20%28double-precision%29) (InputAction :type Input%20Action%20Object%20Reference :default "/Game/Blueprints/Player/Input/Player1/I_JumpP1.I_JumpP1"))
  (:Started
    (Class|PlayerDuoController|JumpP1))
  (:Canceled
    (Class|PlayerDuoController|StopJumpP1)))

(event Input|EnhancedActionEvents|EnhancedInputActionI_JumpP2
  (params (ActionValue :type Boolean) (ElapsedSeconds :type Float%20%28double-precision%29) (TriggeredSeconds :type Float%20%28double-precision%29) (InputAction :type Input%20Action%20Object%20Reference :default "/Game/Blueprints/Player/Input/Player2/I_JumpP2.I_JumpP2"))
  (:Started
    (Class|PlayerDuoController|JumpP2))
  (:Canceled
    (Class|PlayerDuoController|StopJumpP2)))

(event EventBeginPlay
  (Input|AddMappingContext (PlayerController|LocalPlayerSubsystems|GetEnhancedInputLocalPlayerSubsystem) "/Game/Blueprints/Player/Input/IM_Game.IM_Game" 0 "(bIgnoreAllPressedKeysUntilRelease=True,bForceImmediately=False)")
  (Class|PlayerDuoController|SpawnPlayerPawn (Math|Transform|MakeTransform "0.000000,0.000000,10.000000" "0.000000,90.000000,0.000000") true)
  (Class|PlayerDuoController|SpawnPlayerPawn (Math|Transform|MakeTransform "0.000000,100.000000,10.000000" "0.000000,90.000000,0.000000") false)
  (bind _returnvalue (Actor|GetActorOfClass "/Game/Blueprints/Camera/BP_InteligentCamera.BP_InteligentCamera_C"))
  (Game|Player|SetViewTargetwithBlend _returnvalue 0.0 "VTBlend_Linear" 0.0 false))

(fn ConstructionScript)