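; A platform that disappears shortly after the player pawn touches it and respawns later.
; Overlap on the Colision component sets a guard flag, waits DisapearTime, then hides the actor and turns off the Cube mesh collision.
; After RespawnTime it shows the actor, restores collision and clears the flag so it can trigger again.
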(event OnComponentBeginOverlap(Colision)
  (params (OverlappedComponent :type Primitive%20Component%20Object%20Reference) (OtherActor :type Actor%20Object%20Reference) (OtherComp :type Primitive%20Component%20Object%20Reference) (OtherBodyIndex :type Integer) (bFromSweep :type Boolean) (SweepResult :type Hit%20Result%20Structure%20%28by%20ref%29))
  (if (not (Variables|Default|GetPlatform%20actived))
    (Utilities|Casting|CastToPlayerPawn OtherActor)
    (Variables|Default|SetPlatform%20actived true)
    (Utilities|FlowControl|Delay (Variables|Default|GetDisapear%20Time))
    (Rendering|SetActorHiddenInGame true)
    (Collision|SetCollisionEnabled (Variables|Default|GetCube) "NoCollision")
    (Utilities|FlowControl|Delay (Variables|Default|GetRespawn%20Time))
    (Rendering|SetActorHiddenInGame false)
    (Collision|SetCollisionEnabled (Variables|Default|GetCube) "QueryAndPhysics")
    (Variables|Default|SetPlatform%20actived false)))

(event OnComponentEndOverlap(Colision)
  (params (OverlappedComponent :type Primitive%20Component%20Object%20Reference) (OtherActor :type Actor%20Object%20Reference) (OtherComp :type Primitive%20Component%20Object%20Reference) (OtherBodyIndex :type Integer)))

(event EventBeginPlay)

(event Collision|EventActorBeginOverlap
  (params (OtherActor :type Actor%20Object%20Reference)))

(event EventTick
  (params (DeltaSeconds :type Float%20%28single-precision%29)))

(fn ConstructionScript)